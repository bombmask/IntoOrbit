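; Player pawn for an orbit simulation that can fly to and ride clicked actors, and spawns batches of MyOrbitBody on R using config-driven spawn options.
; Left click traces from the camera and binds a lerp event to a dispatcher called every Tick, easing toward the target's live location.
; Once within tolerance, the pawn unbinds the lerp and snap-attaches to the target.
; Right click detaches and cancels any movement.
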(event `LerpTo_Event`
  (params (Dt :type "Float (double-precision)"))
  (bind _out (`/Game/OrbitContent/Blueprints/OrbitMacros.AddNumberByRef` (`self.DT`) Dt))
  (`|ExecutionSequence`
    (:`then_0`
      (`/Engine/EditorBlueprintResources/StandardMacros.DoOnce` false :!label _label
        (:`Completed`
          (set `self.Start` (`self.K2_GetActorLocation`))
          (set `self.DT` 0.0))))
    (:`then_1`
      (`self.K2_SetActorLocation` (`KismetMathLibrary.VLerp` (`self.K2_GetActorLocation`) (`self.GetAttachLocation`) (/ _out 1.75)) false true))
    (:`then_2`
      (if (== (`self.GetAttachLocation`) (`self.K2_GetActorLocation`) :`ErrorTolerance` 1.0)
        (clear `self.LerpTo`)
        (`self.K2_AttachRootComponentToActor` (`self.CurrentAttach`) "None" "SnapToTarget")
        (goto _label :!via `Reset`)))))

(event `Key|LeftMouseButton`
  (params (Key :type "Key Structure" :default "AnyKey"))
  (bind (_start _end) (`FireUtilBPLibrary.TraceVectorLength` (`PlayerCameraManager.TransformComponent` (`GameplayStatics.GetPlayerCameraManager` 0)) "X" 10000.0))
  (:`Pressed`
    (bind (_outhit _returnvalue) (`KismetSystemLibrary.LineTraceSingleForObjects` _start _end (`|MakeArray` "ObjectTypeQuery2" "ObjectTypeQuery1" :!type "EObjectTypeQuery Enum") false (`|MakeArray` (`self.CurrentAttach`))))
    (if _returnvalue
      (bind (_bblockinghit _binitialoverlap _time _location _impactpoint _normal _impactnormal _physmat _hitactor) (`GameplayStatics.BreakHitResult` _outhit))
      (if (`KismetSystemLibrary.IsValid` _hitactor)
        (set `self.CurrentAttach` _hitactor)
        (add `self.LerpTo` (delegate `LerpTo_Event`))))))

(event `Key|RightMouseButton`
  (params (Key :type "Key Structure" :default "AnyKey"))
  (:`Pressed`
    (`self.DetachRootComponentFromParent` true)
    (set `self.CurrentAttach` null)
    (clear `self.LerpTo`)))

(event `self.ReceiveTick`
  (params (DeltaSeconds :type "Float (single-precision)"))
  (`self.LerpTo` DeltaSeconds))

(event `Key|R`
  (params (Key :type "Key Structure" :default "AnyKey"))
  (bind (_config_densitymin _config_densitymax _config_usedensityrandom _config_initalvelocitydirection _config_coneangle _config_useconerandom _config_speedmin _config_speedmax _config_userandomspeed) (break `/Game/OrbitContent/Blueprints/SpawnConfig` (`self.Config`)))
  (bind (_config_densitymin_2 _config_densitymax_2 _config_usedensityrandom_2 _config_initalvelocitydirection_2 _config_coneangle_2 _config_useconerandom_2 _config_speedmin_2 _config_speedmax_2 _config_userandomspeed_2 _config_boxsize _config_boxorigin) (break `/Game/OrbitContent/Blueprints/SpawnConfig` (`self.Config`)))
  (bind (_config_densitymin_3 _config_densitymax_3 _config_usedensityrandom_3 _config_initalvelocitydirection_3 _config_coneangle_3 _config_useconerandom_3 _config_speedmin_3 _config_speedmax_3 _config_userandomspeed_3 _config_boxsize_2 _config_boxorigin_2 _config_numbertospawn) (break `/Game/OrbitContent/Blueprints/SpawnConfig` (`self.Config`)))
  (:`Pressed`
    (for _ (range (+ _config_numbertospawn 1))
      (`|SpawnActorFromClass` "/Game/OrbitContent/Blueprints/MyOrbitBody.MyOrbitBody_C" (`KismetMathLibrary.Conv_VectorToTransform` (`KismetMathLibrary.RandomPointInBoundingBox` _config_boxorigin (`KismetMathLibrary.Conv_DoubleToVector` _config_boxsize))) "Undefined" "OverrideRootScale" null (select `bool` _config_usedensityrandom :`false` _config_densitymin :`true` (`KismetMathLibrary.RandomFloatInRange` _config_densitymin _config_densitymax)) true (* (select `bool` _config_useconerandom :`false` (`KismetMathLibrary.RandomUnitVectorInCone` _config_initalvelocitydirection _config_coneangle) :`true` (1.0 0.0 0.0)) (select `bool` _config_userandomspeed :`false` _config_speedmin :`true` (`KismetMathLibrary.RandomFloatInRange` _config_speedmin _config_speedmax)))))))

(fn `UserConstructionScript`)