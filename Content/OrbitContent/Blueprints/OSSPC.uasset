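; OSSPC is a player controller that sets up the on-screen UI and handles pausing.
; On BeginPlay it adds a WidgetHandler widget as the reticle and creates a centered Pause widget, kept off screen until needed.
; The PauseButton input or a ToggleViewport event toggles that menu, switching between UI-only and game-only input and showing or hiding the cursor.
; The toggle does not pause the game itself.
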(event `self.ReceiveBeginPlay`
  (bind _pauseui (`self.PauseUI`))
  (bind _returnvalue (`|CreateWidget` "/Game/OrbitContent/GUI/WidgetHandler.WidgetHandler_C"))
  (`UserWidget.AddToViewport` _returnvalue 0)
  (bind _returnvalue_2 (`|CreateWidget` "/Game/OrbitContent/GUI/Pause.Pause_C" self))
  (`|ExecutionSequence`
    (:`then_0`
      (set `self.PauseUI` _returnvalue_2))
    (:`then_1`
      (`UserWidget.SetAlignmentInViewport` _pauseui (0.5 0.5)))
    (:`then_2`
      (`UserWidget.SetAnchorsInViewport` _pauseui (make `Anchors` (0.5 0.5) (0.5 0.5))))))

(event `InputAction|PauseButton`
  (params (Key :type "Key Structure" :default "AnyKey"))
  (bind _pauseui (`self.PauseUI`))
  (:`Pressed`
    (if (`Widget.IsInViewport` (`self.PauseUI`)) :!label _label
      (`Widget.RemoveFromParent` (`self.PauseUI`))
      (`WidgetBlueprintLibrary.SetInputMode_GameOnly` self)
      (set `self.bShowMouseCursor` false)
      (else
        (`UserWidget.AddToViewport` _pauseui 0)
        (`WidgetBlueprintLibrary.SetInputMode_UIOnlyEx` self _pauseui)
        (set `self.bShowMouseCursor` true)))))

(event `ToggleViewport`
  (goto _label))

(fn `UserConstructionScript`)